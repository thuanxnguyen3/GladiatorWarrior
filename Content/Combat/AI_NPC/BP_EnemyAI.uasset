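; BP_EnemyAI is an enemy character Blueprint that reacts to taking damage.
; AnyDamage plays a random montage from HitAnims, then launches the enemy along the facing direction of player 0's BP_ThirdPersonCharacter, whatever the damage source.
; An unconnected fragment would set the "hasSeenPlayer?" Blackboard key on a "Player" tag check, but it never runs.
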(event `self.ReceiveAnyDamage`
  (params (Damage :type "Float (single-precision)") (DamageType :type "DamageType Object Reference") (InstigatedBy :type "Controller Object Reference") (DamageCauser :type "Actor Object Reference"))
  (`self.PlayAnimMontage` (`|GetArrayItem` (`self.Hit Anims`) (`KismetMathLibrary.RandomIntegerInRange` 0 (- (`KismetArrayLibrary.Array_Length` (`self.Hit Anims`)) 1))))
  (bind _asbp_third_person_character (cast `/Game/ThirdPerson/Blueprints/BP_ThirdPersonCharacter` (`GameplayStatics.GetPlayerCharacter` 0)))
  (`self.LaunchCharacter` (* (`KismetMathLibrary.GetForwardVector` (`self.K2_GetActorRotation` _asbp_third_person_character)) 500.0)))

(fn `UserConstructionScript`)