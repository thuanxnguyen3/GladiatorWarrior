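; BP_AISpawner is a wave-style spawner that starts spawning AI after a delay from BeginPlay.
; SpawnAI loops over the current count, spawning actors with yaw taken from the spawner-to-player look-at rotation, and re-calls itself if that count is zero or less.
; OnAIDeath decrements the count; at zero it doubles the base count for a new wave, otherwise it spawns the remaining count again.
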(event `self.ReceiveBeginPlay`
  (`KismetSystemLibrary.Delay` 11.52)
  (`self.SpawnAI` (`self.Current Spawn Count`)))

(event `SpawnAI`
  (params (`Current Spawn Count` :type Integer))
  (for _ (range `Current Spawn Count`)
    (`|SpawnActorFromClass` "/Game/Combat/AI_NPC/BP_EnemyAI.BP_EnemyAI_C" (`KismetMathLibrary.MakeTransform` (`self.Spawn Transform Location`) (`KismetMathLibrary.MakeRotator` 0.0 0.0 (.yaw (`KismetMathLibrary.FindLookAtRotation` (`self.K2_GetActorLocation`) (`self.K2_GetActorLocation` (`GameplayStatics.GetPlayerCharacter` 0)))))) "Undefined" "MultiplyWithRoot" null null))
  (if (<= (`self.Current Spawn Count`) 0)
    (`self.SpawnAI` (`self.Current Spawn Count`))))

(event `OnAIDeath`
  (bind _result (`/Engine/EditorBlueprintResources/StandardMacros.DecrementFloat` (`KismetMathLibrary.Conv_IntToDouble` (`self.Current Spawn Count`)))
    (:`  `
      (bind _output_get (set `self.Current Spawn Count` (`KismetMathLibrary.FTrunc` _result)))
      (if (<= _output_get 0)
        (bind _output_get_2 (set `self.BaseSpawnCount` (* (`self.BaseSpawnCount`) 2)))
        (bind _output_get_3 (set `self.Current Spawn Count` _output_get_2))
        (`self.SpawnAI` _output_get_3)
        (else
          (`self.SpawnAI` (`self.Current Spawn Count`)))))))

(fn `UserConstructionScript`)