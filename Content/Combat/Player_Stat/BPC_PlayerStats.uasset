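; Stats component that tracks health and stamina for BP_ThirdPersonCharacter, and is also built to work on BP_EnemyAI.
; One tick after BeginPlay it casts its owner, sets IsPlayer and initializes the HUD or enemy health bar.
; Decrease functions report depletion, while Increase functions cap current values or raise maximums, all refreshing UI directly.
; Only DecreaseHealth updates enemy UI after startup; other functions target the player HUD.
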(event `self.ReceiveBeginPlay`
  (`KismetSystemLibrary.DelayUntilNextTick`)
  (bind _asbp_third_person_character (cast `/Game/ThirdPerson/Blueprints/BP_ThirdPersonCharacter` (`self.GetOwner`))
    (:`then`
      (set `self.Player Character BP` _asbp_third_person_character)
      (set `self.IsPlayer` true)
      (`ProgressBar.SetPercent` (`/Game/Combat/Player_Stat/WB_HUD.StaminaBar` (`/Game/ThirdPerson/Blueprints/BP_ThirdPersonCharacter.HUD Widget` (`self.Player Character BP`))) (/ (`self.Stamina`) (`self.Max Stamina`))))
    (:`CastFailed`
      (bind _asbp_enemy_ai (cast `/Game/Combat/AI_NPC/BP_EnemyAI` (`self.GetOwner`)))
      (set `self.Enemy AI BP` _asbp_enemy_ai)
      (set `self.IsPlayer` false)))
  (`ProgressBar.SetPercent` (select `bool` (`self.IsPlayer`) :`false` (`/Game/Combat/AI_NPC/WB_EnemyAIHealth.HealthBar` (`/Game/Combat/AI_NPC/BP_EnemyAI.Health Bar UI` (`self.Enemy AI BP`))) :`true` (`/Game/Combat/Player_Stat/WB_HUD.HealthBar` (`/Game/ThirdPerson/Blueprints/BP_ThirdPersonCharacter.HUD Widget` (`self.Player Character BP`)))) (/ (`self.Health`) (`self.Max Health`)))
  (`TextBlock.SetText` (select `bool` (`self.IsPlayer`) :`false` (`/Game/Combat/AI_NPC/WB_EnemyAIHealth.HealthText` (`/Game/Combat/AI_NPC/BP_EnemyAI.Health Bar UI` (`self.Enemy AI BP`))) :`true` (`/Game/Combat/Player_Stat/WB_HUD.HealthText` (`/Game/ThirdPerson/Blueprints/BP_ThirdPersonCharacter.HUD Widget` (`self.Player Character BP`)))) (`KismetTextLibrary.Conv_DoubleToText` (`self.Health`) "HalfToEven")))

(fn `Decrease Health`
  (params (Damage :type "Float (double-precision)"))
  (returns (`Is Player Dead?` :type Boolean))
  (if (not (<= (`self.Health`) 0.0))
    (bind _output_get (set `self.Health` (- (`self.Health`) Damage)))
    (`ProgressBar.SetPercent` (select `bool` (`self.IsPlayer`) :`false` (`/Game/Combat/AI_NPC/WB_EnemyAIHealth.HealthBar` (`/Game/Combat/AI_NPC/BP_EnemyAI.Health Bar UI` (`self.Enemy AI BP`))) :`true` (`/Game/Combat/Player_Stat/WB_HUD.HealthBar` (`/Game/ThirdPerson/Blueprints/BP_ThirdPersonCharacter.HUD Widget` (`self.Player Character BP`)))) (/ _output_get (`self.Max Health`)))
    (`TextBlock.SetText` (select `bool` (`self.IsPlayer`) :`false` (`/Game/Combat/AI_NPC/WB_EnemyAIHealth.HealthText` (`/Game/Combat/AI_NPC/BP_EnemyAI.Health Bar UI` (`self.Enemy AI BP`))) :`true` (`/Game/Combat/Player_Stat/WB_HUD.HealthText` (`/Game/ThirdPerson/Blueprints/BP_ThirdPersonCharacter.HUD Widget` (`self.Player Character BP`)))) (`KismetTextLibrary.Conv_DoubleToText` (`self.Health`) "HalfToEven"))
    (if (<= (`self.Health`) 0.0)
      _
      (else
        (return false))))
  (return true))

(fn `Decrease Stamina`
  (params (`Stamina Depleted` :type "Float (double-precision)"))
  (returns (`No Stamina Left` :type Boolean))
  (if (not (<= (`self.Stamina`) 0.0))
    (set `self.Stamina` (- (`self.Stamina`) `Stamina Depleted`))
    (`ProgressBar.SetPercent` (`/Game/Combat/Player_Stat/WB_HUD.StaminaBar` (`/Game/ThirdPerson/Blueprints/BP_ThirdPersonCharacter.HUD Widget` (`self.Player Character BP`))) (/ (`self.Stamina`) (`self.Max Stamina`)))
    (if (<= (`self.Stamina`) 0.0)
      _
      (else
        (return false))))
  (return true))

(fn `Increase Health`
  (params (`Added Health` :type "Float (double-precision)"))
  (bind _hud_widget (`/Game/ThirdPerson/Blueprints/BP_ThirdPersonCharacter.HUD Widget` (`self.Player Character BP`)))
  (set `self.Health` (+ (`self.Health`) `Added Health`))
  (if (> (`self.Health`) (`self.Max Health`))
    (set `self.Health` (`self.Max Health`)))
  (`ProgressBar.SetPercent` (`/Game/Combat/Player_Stat/WB_HUD.HealthBar` _hud_widget) (/ (`self.Health`) (`self.Max Health`)))
  (`TextBlock.SetText` (`/Game/Combat/Player_Stat/WB_HUD.HealthText` _hud_widget) (`KismetTextLibrary.Conv_DoubleToText` (`self.Health`) "HalfToEven")))

(fn `Increase Max Health`
  (params (`Increase HP` :type "Float (double-precision)"))
  (bind _hud_widget (`/Game/ThirdPerson/Blueprints/BP_ThirdPersonCharacter.HUD Widget` (`self.Player Character BP`)))
  (set `self.Max Health` (+ (`self.Max Health`) `Increase HP`))
  (`ProgressBar.SetPercent` (`/Game/Combat/Player_Stat/WB_HUD.HealthBar` _hud_widget) (/ (`self.Health`) (`self.Max Health`)))
  (`TextBlock.SetText` (`/Game/Combat/Player_Stat/WB_HUD.HealthText` _hud_widget) (`KismetTextLibrary.Conv_DoubleToText` (`self.Health`) "HalfToEven")))

(fn `Increase Max Stamina`
  (params (`Added Stamina` :type "Float (double-precision)"))
  (set `self.Max Stamina` (+ (`self.Max Stamina`) `Added Stamina`))
  (`ProgressBar.SetPercent` (`/Game/Combat/Player_Stat/WB_HUD.StaminaBar` (`/Game/ThirdPerson/Blueprints/BP_ThirdPersonCharacter.HUD Widget` (`self.Player Character BP`))) (/ (`self.Stamina`) (`self.Max Stamina`))))

(fn `Increase Stamina`
  (params (`Added Stamina` :type "Float (double-precision)"))
  (set `self.Stamina` (+ (`self.Stamina`) `Added Stamina`))
  (if (> (`self.Stamina`) (`self.Max Stamina`))
    (set `self.Stamina` (`self.Max Stamina`)))
  (`ProgressBar.SetPercent` (select `bool` (`self.IsPlayer`) :`true` (`/Game/Combat/Player_Stat/WB_HUD.StaminaBar` (`/Game/ThirdPerson/Blueprints/BP_ThirdPersonCharacter.HUD Widget` (`self.Player Character BP`)))) (/ (`self.Stamina`) (`self.Max Stamina`))))